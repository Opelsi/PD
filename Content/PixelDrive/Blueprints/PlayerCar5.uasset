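; PlayerCar5 is a player car Blueprint whose Ultra ability puts it on temporary autopilot.
; Ultra sets QuestDone, disables the HUD's left and right buttons, enables AutoPilot for UltraDuration, then restores both.
; During autopilot, a FrontCar overlap with another Car shifts this car sideways in X, randomly from the center lane or back toward center from side lanes.
; The CrushCol overlap only casts to Coin, with no further action.
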(event OnComponentBeginOverlap(CrushCol)
  (params (OverlappedComponent :type Primitive%20Component%20Object%20Reference) (OtherActor :type Actor%20Object%20Reference) (OtherComp :type Primitive%20Component%20Object%20Reference) (OtherBodyIndex :type Integer) (bFromSweep :type Boolean) (SweepResult :type Hit%20Result%20Structure%20%28by%20ref%29))
  (Utilities|Casting|CastToCoin OtherActor))

(event OnComponentBeginOverlap(FrontCar)
  (params (OverlappedComponent :type Primitive%20Component%20Object%20Reference) (OtherActor :type Actor%20Object%20Reference) (OtherComp :type Primitive%20Component%20Object%20Reference) (OtherBodyIndex :type Integer) (bFromSweep :type Boolean) (SweepResult :type Hit%20Result%20Structure%20%28by%20ref%29))
  (bind _returnvalue (Transformation|GetActorLocation))
  (bind _returnvalue_2 (Math|Random|RandomInteger 1))
  (bind _randomx (Variables|Default|GetRandomX))
  (bind _output (Utilities|Array|Get(acopy) _randomx _returnvalue_2))
  (if (Variables|Default|GetAutoPilot)
    (Utilities|Casting|CastToCar OtherActor)
    (if (== (.x _returnvalue) 0.0)
      (Development|PrintString (Utilities|String|ToString(Float) _output))
      (Transformation|AddActorWorldOffset (Math|Vector|MakeVector _output 0.0 0.0))
      (elif (== (.x _returnvalue) -32.0)
        (Transformation|AddActorWorldOffset (Math|Vector|MakeVector 32.0 0.0 0.0))
        (else
          (Transformation|AddActorWorldOffset (Math|Vector|MakeVector -32.0 0.0 0.0)))))))

(event EventBeginPlay
  (|CallParentFunction)
  (bind _asgame_hud (Utilities|Casting|CastToGameHud (HUD|GetHUD (Game|GetPlayerController 0))))
  (Variables|Default|SetGameHud _asgame_hud))

(event Collision|EventActorBeginOverlap
  (params (OtherActor :type Actor%20Object%20Reference)))

(event EventTick
  (params (DeltaSeconds :type Float%20%28single-precision%29))
  (|CallParentFunction DeltaSeconds))

(event EventUltra
  (bind _gamehud (Variables|Default|GetGameHud))
  (bind _gamestartedwidget (Variables|/Game/PixelDrive/Blueprints/GameHud.GameHud_C|GetGameStartedWidget _gamehud))
  (bind _leftbutton (Variables|/Game/PixelDrive/Blueprints/GameStarted.GameStarted_C|GetLeftButton _gamestartedwidget))
  (bind _rightbutton (Variables|/Game/PixelDrive/Blueprints/GameStarted.GameStarted_C|GetRightButton _gamestartedwidget))
  (Variables|Default|SetQuest%20Done true)
  (Widget|SetIsEnabled _rightbutton false)
  (Widget|SetIsEnabled _leftbutton false)
  (Variables|Default|SetAutoPilot true)
  (Utilities|FlowControl|Delay (Variables|Default|GetUltraDuration))
  (Widget|SetIsEnabled _rightbutton true)
  (Widget|SetIsEnabled _leftbutton true)
  (Variables|Default|SetAutoPilot false))

(fn ConstructionScript
  (|CallParentFunction))