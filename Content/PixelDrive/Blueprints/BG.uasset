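; BG is a background actor for the PixelDrive car game that scrolls along the world Z axis.
; On BeginPlay it casts the game mode to CarGamemode and caches the reference.
; Each Tick it offsets itself without sweep by the game mode's Speed scaled by delta time, or prints a debug string if that reference is invalid.
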(event EventBeginPlay
  (bind _ascar_gamemode (Utilities|Casting|CastToCarGamemode (Game|GetGameMode)))
  (Variables|Default|SetGameMode _ascar_gamemode))

(event Collision|EventActorBeginOverlap
  (params (OtherActor :type Actor%20Object%20Reference)))

(event EventTick
  (params (DeltaSeconds :type Float%20%28single-precision%29))
  (bind _gamemode (Variables|Default|GetGameMode))
  (if (Utilities|IsValid _gamemode)
    (Transformation|AddActorWorldOffset self (* (Math|Vector|MakeVector 0.0 0.0 (Variables|/Game/PixelDrive/Blueprints/CarGamemode.CarGamemode_C|GetSpeed _gamemode)) DeltaSeconds))
    (else
      (Development|PrintString "Hello"))))

(fn ConstructionScript)