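; Car actor for a 2D Paper2D driving game that picks a random sprite and its CarGamemode reference in the construction script.
; Each tick it moves along world Z at half the game mode's Speed, or at full Speed while Stopped, apparently matching the world scroll.
; Box overlap with an Obstacle sets Stopped until the overlap ends, while overlap with another Car destroys that other car.
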(event OnComponentBeginOverlap(Box)
  (params (OverlappedComponent :type Primitive%20Component%20Object%20Reference) (OtherActor :type Actor%20Object%20Reference) (OtherComp :type Primitive%20Component%20Object%20Reference) (OtherBodyIndex :type Integer) (bFromSweep :type Boolean) (SweepResult :type Hit%20Result%20Structure%20%28by%20ref%29))
  (Utilities|Casting|CastToObstacle OtherActor
    (:then
      (Variables|Default|SetStopped true))
    (:CastFailed
      (Utilities|Casting|CastToCar OtherActor)
      (Actor|DestroyActor OtherActor))))

(event OnComponentEndOverlap(Box)
  (params (OverlappedComponent :type Primitive%20Component%20Object%20Reference) (OtherActor :type Actor%20Object%20Reference) (OtherComp :type Primitive%20Component%20Object%20Reference) (OtherBodyIndex :type Integer))
  (Utilities|Casting|CastToObstacle OtherActor)
  (Variables|Default|SetStopped false))

(event EventBeginPlay)

(event Collision|EventActorBeginOverlap
  (params (OtherActor :type Actor%20Object%20Reference)))

(event EventTick
  (params (DeltaSeconds :type Float%20%28single-precision%29))
  (if (Variables|Default|GetStopped)
    (Variables|Default|SetSpeed (Variables|/Game/PixelDrive/Blueprints/CarGamemode.CarGamemode_C|GetSpeed (Variables|Default|GetGamemode)))
    (else
      (Variables|Default|SetSpeed (/ (Variables|/Game/PixelDrive/Blueprints/CarGamemode.CarGamemode_C|GetSpeed (Variables|Default|GetGamemode)) 2.0))))
  (Transformation|AddActorWorldOffset self (* (Math|Vector|MakeVector 0.0 0.0 (Variables|Default|GetSpeed)) DeltaSeconds)))

(fn ConstructionScript
  (bind _cars (Variables|Default|GetCars))
  (bind _ascar_gamemode (Utilities|Casting|CastToCarGamemode (Game|GetGameMode)))
  (Variables|Default|SetGamemode _ascar_gamemode)
  (Rendering|Components|Sprite|SetSprite (Variables|Default|GetPaperSprite) (Utilities|Array|Get(acopy) _cars (Math|Random|RandomInteger (Utilities|Array|Length _cars)))))