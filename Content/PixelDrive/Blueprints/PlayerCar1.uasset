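; PlayerCar1 is a player car Blueprint in PixelDrive with its own Ultra ability.
; On BeginPlay it loads player info and shows itself with crush collision enabled only if it is the last selected car, otherwise hiding and disabling that collision.
; Ultra sets QuestDone, then temporarily stops car spawning and applies a large negative player multiplier on the GameMode, restoring both after UltraDuration.
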(event EventBeginPlay
  (|CallParentFunction)
  (bind _lastcar (CallFunction|LoadPlayerInfo))
  (if (!= _lastcar "PlayerCar1_C")
    (Rendering|SetActorHiddenInGame true)
    (Collision|SetCollisionEnabled (Variables|Default|GetCrushCol) "NoCollision")
    (else
      (Rendering|SetActorHiddenInGame false)
      (Collision|SetCollisionEnabled (Variables|Default|GetCrushCol) "QueryAndPhysics"))))

(event Collision|EventActorBeginOverlap
  (params (OtherActor :type Actor%20Object%20Reference))
  (|CallParentFunction OtherActor) ; This node is disabled and will not be called.\nDrag off pins to build functionality.
)

(event EventTick
  (params (DeltaSeconds :type Float%20%28single-precision%29))
  (|CallParentFunction DeltaSeconds) ; This node is disabled and will not be called.\nDrag off pins to build functionality.
)

(event EventUltra
  (bind _gamemode (Variables|Default|GetGameMode))
  (Variables|Default|SetQuest%20Done true)
  (Variables|/Game/PixelDrive/Blueprints/CarGamemode.CarGamemode_C|SetPlayerMultiplier _gamemode -8.0)
  (Variables|Default|SetSpawnCars false)
  (Utilities|FlowControl|Delay (Variables|Default|GetUltraDuration))
  (Variables|/Game/PixelDrive/Blueprints/CarGamemode.CarGamemode_C|SetPlayerMultiplier _gamemode 1.0)
  (Variables|Default|SetSpawnCars true))

(fn ConstructionScript
  (|CallParentFunction))