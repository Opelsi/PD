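; Obstacle actor for the PixelDrive car game that moves at the game mode's speed, either standing or crossing horizontally.
; Construction randomly picks the type, then sets a biome-dependent sprite, plus an X multiplier for horizontal Suburb and Field obstacles.
; BeginPlay derives facing from spawn X, and Start turns it into signed X speed.
; Tick applies movement, flipping horizontal sprites on a delayed FlipFlop as simple animation.
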(event Custom|Start
  (bind _gamemode (Variables|Default|GetGamemode))
  (bind _xmultiplier (Variables|Default|GetXMultiplier))
  (bind _speed (Variables|/Game/PixelDrive/Blueprints/CarGamemode.CarGamemode_C|GetSpeed _gamemode))
  (bind _returnvalue (* _speed _xmultiplier))
  (if (Variables|Default|GetGoRight)
    (Variables|Default|SetXSpeed (* _returnvalue -1.0))
    (else
      (Variables|Default|SetXSpeed _returnvalue))))

(event EventBeginPlay
  (bind _returnvalue (Transformation|GetActorLocation))
  (bind _papersprite (Variables|Default|GetPaperSprite))
  (if (== (.x _returnvalue) 0.0)
    (Variables|Default|SetGoRight (Math|Random|RandomBool))
    (elif (== (.x _returnvalue) -32.0)
      (Variables|Default|SetGoRight true)
      (else
        (Variables|Default|SetGoRight false))))
  (if (Variables|Default|GetGoRight)
    (Transformation|SetWorldRotation _papersprite "0, 0, 0" false false)
    (else
      (Transformation|SetWorldRotation _papersprite "180.000000, 0, 0" false false))))

(event Collision|EventActorBeginOverlap
  (params (OtherActor :type Actor%20Object%20Reference)))

(event EventTick
  (params (DeltaSeconds :type Float%20%28single-precision%29))
  (bind _gamemode (Variables|Default|GetGamemode))
  (bind _papersprite (Variables|Default|GetPaperSprite))
  (if (Utilities|IsValid _gamemode)
    (Transformation|AddActorWorldOffset (* (Math|Vector|MakeVector (Variables|Default|GetXSpeed) 0.0 (Variables|/Game/PixelDrive/Blueprints/CarGamemode.CarGamemode_C|GetSpeed _gamemode)) DeltaSeconds))
    (switch Utilities|FlowControl|Switch|SwitchonObstacles (Variables|Default|GetType)
      (:NewEnumerator0
        (Utilities|FlowControl|Delay 0.25)
        (Utilities|FlowControl|FlipFlop
          (:A
            (Transformation|SetRelativeScale3D _papersprite "1.000000,1.000000,-1.000000"))
          (:B
            (Transformation|SetRelativeScale3D _papersprite "1.000000,1.000000,1.000000")))))))

(fn ConstructionScript
  (bind _obstacles (Variables|Default|GetObstacles))
  (bind _papersprite (Variables|Default|GetPaperSprite))
  (bind _ascar_gamemode (Utilities|Casting|CastToCarGamemode (Game|GetGameMode)))
  (Variables|Default|SetGamemode _ascar_gamemode)
  (bind _output_get (Variables|Default|SetType (Utilities|Array|Get(acopy) _obstacles (Math|Random|RandomInteger (Utilities|Array|Length _obstacles)))))
  (Variables|Default|SetRandom (Math|Random|RandomInteger (Utilities|Array|Length (Variables|Default|GetSpritesType))))
  (switch Utilities|FlowControl|Switch|SwitchonObstacles _output_get
    (:NewEnumerator0
      (Variables|Default|SetSpritesType (Variables|Default|GetHorizontalSprites))
      (switch Utilities|FlowControl|Switch|SwitchonBiomes (Variables|/Game/PixelDrive/Blueprints/CarGamemode.CarGamemode_C|GetNewBiome (Variables|Default|GetGamemode))
        (:NewEnumerator0
          (Rendering|Components|Sprite|SetSprite _papersprite "/Game/PixelDrive/Textures/Textures190318_Bicycle_0.Textures190318_Bicycle_0" :!label _label))
        (:NewEnumerator1
          (goto _label))
        (:NewEnumerator2
          (Variables|Default|SetXMultiplier (Utilities|Array|Get(acopy) (Variables|Default|GetXMultipliers) (Variables|Default|GetRandom)) :!label _label_2)
          (Rendering|Components|Sprite|SetSprite _papersprite (Utilities|Array|Get(acopy) (Variables|Default|GetSpritesType) (Variables|Default|GetRandom)) :!label _label_3))
        (:NewEnumerator3
          (goto _label_2))))
    (:NewEnumerator1
      (Variables|Default|SetSpritesType (Variables|Default|GetStandSprites))
      (switch Utilities|FlowControl|Switch|SwitchonBiomes (Variables|/Game/PixelDrive/Blueprints/CarGamemode.CarGamemode_C|GetNewBiome (Variables|Default|GetGamemode))
        (:NewEnumerator0
          _)
        (:NewEnumerator1
          _)
        (:NewEnumerator2
          (goto _label_3))
        (:NewEnumerator3
          (goto _label_3)))
      (Rendering|Components|Sprite|SetSprite _papersprite "/Game/PixelDrive/Textures/Textures190318_Pit_0.Textures190318_Pit_0"))))