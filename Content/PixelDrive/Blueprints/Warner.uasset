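; Warner is a PixelDrive actor that flashes a warning widget at a given line, likely a driving lane.
; Its Warn event converts the line index into a world X position on a fixed-spacing grid, keeping the widget's Y and Z.
; It then shows the widget and hides it after a shortened fraction of the supplied delay.
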(event Custom|Warn
  (params (Line :type Integer) (Delay :type Float%20%28single-precision%29))
  (bind _widget (Variables|Default|GetWidget))
  (bind _returnvalue (Transformation|GetWorldLocation _widget))
  (bind (_x _y _z) (Math|Vector|BreakVector _returnvalue))
  (Transformation|SetWorldLocation _widget (Math|Vector|MakeVector (Math|Conversions|ToFloat(Integer) (+ (* Line 32) -32)) _y _z) false false)
  (Rendering|SetVisibility _widget true false)
  (Utilities|FlowControl|Delay (/ Delay 1.5))
  (Rendering|SetVisibility _widget false false))

(event EventBeginPlay)

(event Collision|EventActorBeginOverlap
  (params (OtherActor :type Actor%20Object%20Reference)))

(event EventTick
  (params (DeltaSeconds :type Float%20%28single-precision%29)))

(fn ConstructionScript)