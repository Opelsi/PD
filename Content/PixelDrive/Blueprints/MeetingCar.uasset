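; MeetingCar is a traffic car actor in PixelDrive that destroys the Car it overlaps and plays a hit sound.
; The construction script caches the CarGamemode and gives the Paper2D sprite a random pick from the Sprites array.
; Each tick it moves along world Z at one and a half times the game mode's Speed, scaled by delta time, without sweeping.
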(event OnComponentBeginOverlap(Box)
  (params (OverlappedComponent :type Primitive%20Component%20Object%20Reference) (OtherActor :type Actor%20Object%20Reference) (OtherComp :type Primitive%20Component%20Object%20Reference) (OtherBodyIndex :type Integer) (bFromSweep :type Boolean) (SweepResult :type Hit%20Result%20Structure%20%28by%20ref%29))
  (Utilities|Casting|CastToCar OtherActor)
  (Actor|DestroyActor OtherActor)
  (Audio|PlaySound2D "/Game/PixelDrive/Music/Hit.Hit"))

(event EventBeginPlay)

(event Collision|EventActorBeginOverlap
  (params (OtherActor :type Actor%20Object%20Reference)))

(event EventTick
  (params (DeltaSeconds :type Float%20%28single-precision%29))
  (Transformation|AddActorWorldOffset (* (Math|Vector|MakeVector 0.0 0.0 (* (Variables|/Game/PixelDrive/Blueprints/CarGamemode.CarGamemode_C|GetSpeed (Variables|Default|GetGamemode)) 1.5)) DeltaSeconds)))

(fn ConstructionScript
  (bind _sprites (Variables|Default|GetSprites))
  (bind _ascar_gamemode (Utilities|Casting|CastToCarGamemode (Game|GetGameMode)))
  (Variables|Default|SetGamemode _ascar_gamemode)
  (Rendering|Components|Sprite|SetSprite (Variables|Default|GetPaperSprite) (Utilities|Array|Get(acopy) _sprites (Math|Random|RandomInteger (Utilities|Array|Length _sprites)))))