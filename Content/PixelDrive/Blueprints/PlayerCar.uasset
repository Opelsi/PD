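; Base player car for PixelDrive that handles collisions, coins, health and one random quest per run.
; BeginPlay loads saved coins and highscore and rolls a quest, while Tick measures its progress from GameMode path, speed and coin count.
; Overlaps apply damage, collect coins or detect the target biome; meeting cars kill instantly.
; Death pauses the game, shows the restart menu and writes the SaveGame slot; Ultra is an empty event.
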(event OnComponentBeginOverlap(CrushCol)
  (params (OverlappedComponent :type Primitive%20Component%20Object%20Reference) (OtherActor :type Actor%20Object%20Reference) (OtherComp :type Primitive%20Component%20Object%20Reference) (OtherBodyIndex :type Integer) (bFromSweep :type Boolean) (SweepResult :type Hit%20Result%20Structure%20%28by%20ref%29))
  (bind _gamemode (Variables|Default|GetGameMode))
  (bind _path (Variables|/Game/PixelDrive/Blueprints/CarGamemode.CarGamemode_C|GetPath _gamemode))
  (bind _returnvalue (Math|Float|Truncate _path))
  ;[1 0.2488 0.2289] Collision
  (Utilities|Casting|CastToCar OtherActor
    (:then
      (Actor|DestroyActor OtherActor :!label _label)
      (Audio|PlaySound2D "/Game/PixelDrive/Music/Hit.Hit")
      (if (== (Variables|Default|GetHealth) 1)
        ;;[1 0.01989 0] Death
        (if (> _returnvalue (Variables|Default|GetHighscore)) :!label _label_2
          (Variables|Default|SetHighscore _returnvalue))
        (CallFunction|Die)
        (else
          ;;[1 0.3128 0] Damged
          (bind _output_get (Variables|Default|SetHealth (- (Variables|Default|GetHealth) 1)))
          (Variables|Default|SetAfterCrash true)
          (if (Variables|Default|GetImmortal)
            (if (<= _output_get 3)
              (Variables|Default|SetImmortal false))
            (else
              (Variables|/Game/PixelDrive/Blueprints/CarGamemode.CarGamemode_C|SetSpeed (Variables|Default|GetGameMode) -1e+02)))
          (Utilities|FlowControl|Delay 2.0)
          (Variables|Default|SetAfterCrash false))))
    (:CastFailed
      (Utilities|Casting|CastToObstacle OtherActor
        (:then
          (goto _label))
        (:CastFailed
          (Utilities|Casting|CastToMeetingCar OtherActor
            (:then
              (Audio|PlaySound2D "/Game/PixelDrive/Music/Hit.Hit")
              (goto _label_2))
            (:CastFailed
              (bind _ascoin (Utilities|Casting|CastToCoin OtherActor)
                (:then
                  (Audio|PlaySound2D "/Game/PixelDrive/Music/Coin.Coin")
                  ;;[1 0.9652 0] EarnCoin
                  (Actor|DestroyActor _ascoin)
                  (Variables|Default|SetCoins (+ (Variables|Default|GetCoins) (Variables|Default|GetMoneyMultiplier))))
                (:CastFailed
                  ;;[0.01415 0.8903 1] CheckBiome
                  (bind _asbg (Utilities|Casting|CastToBG OtherActor))
                  (if (Utilities|Enum|Equal(Enum) (Variables|/Game/PixelDrive/Blueprints/BG.BG_C|GetBiome _asbg) (Variables|Default|GetDestination))
                    (Variables|Default|SetCurrentAmount 100)))))))))))

(event Custom|Ultra)

(event EventBeginPlay
  (bind _returnvalue (Math|Random|RandomIntegerinRange 1 6))
  (bind _quests (Variables|Default|GetQuests))
  (bind _possiblebiomes (Variables|Default|GetPossibleBiomes))
  ;[0.1367 0.3032 1] Begin
  (Utilities|FlowControl|Sequence
    (:then_0
      (bind _ascar_gamemode (Utilities|Casting|CastToCarGamemode (Game|GetGameMode)))
      (Variables|Default|SetGameMode _ascar_gamemode)
      (bind (_coins _highscore) (CallFunction|LoadPlayerInfo))
      (bind _output_get (Variables|Default|SetCoins _coins))
      (Variables|Default|SetHighscore _highscore)
      (Variables|Default|SetStartCoins _output_get))
    (:then_1
      (bind _output_get_2 (Variables|Default|SetCurrentType (Utilities|Array|Get(acopy) _quests (Math|Random|RandomInteger (Utilities|Array|Length _quests)))))
      (switch Utilities|FlowControl|Switch|SwitchonQuestType _output_get_2
        (:NewEnumerator0
          (bind _output_get_3 (Variables|Default|SetAmount (* (Math|Random|RandomIntegerinRange 1 4) 15)))
          (Variables|Default|SetCurrentText (Utilities|Text|ToText(String) (Utilities|String|Append "Earn " (Utilities|String|ToString(Integer) _output_get_3) " coins"))))
        (:NewEnumerator1
          (bind _output_get_4 (Variables|Default|SetAmount (* _returnvalue 250)))
          (Variables|Default|SetCurrentText (Utilities|Text|ToText(String) (Utilities|String|Append "Drive " (Utilities|String|ToString(Integer) _output_get_4) " meters"))))
        (:NewEnumerator2
          (bind _output_get_5 (Variables|Default|SetAmount (* _returnvalue 50)))
          (Variables|Default|SetCurrentText (Utilities|Text|ToText(String) (Utilities|String|Append "Drive " (Utilities|String|ToString(Integer) _output_get_5) " meters 
without earning 
a coin"))))
        (:NewEnumerator3
          (bind _output_get_6 (Variables|Default|SetAmount (* (Math|Random|RandomIntegerinRange 1 3) 100)))
          (Variables|Default|SetCurrentText (Utilities|Text|ToText(String) (Utilities|String|Append " Reach " (Utilities|String|ToString(Integer) _output_get_6) " speed"))))
        (:NewEnumerator4
          (bind _output_get_7 (Variables|Default|SetDestination (Utilities|Array|Get(acopy) _possiblebiomes (Math|Random|RandomInteger (Utilities|Array|Length _possiblebiomes)))))
          (Variables|Default|SetCurrentText (Utilities|Text|ToText(String) (Utilities|String|Append "Get into " (Utilities|String|EnumtoString _output_get_7))))
          (Variables|Default|SetAmount 100))))))

(event EventTick
  (params (DeltaSeconds :type Float%20%28single-precision%29))
  (bind _gamemode (Variables|Default|GetGameMode))
  (bind _path (Variables|/Game/PixelDrive/Blueprints/CarGamemode.CarGamemode_C|GetPath _gamemode))
  (bind _returnvalue (Math|Float|Truncate _path))
  ;[1 0.1583 0.9096] Tick
  (if (not (Variables|Default|GetQuest%20Done))
    (switch Utilities|FlowControl|Switch|SwitchonQuestType (Variables|Default|GetCurrentType)
      (:NewEnumerator0
        (Variables|Default|SetCurrentAmount (- (Variables|Default|GetCoins) (Variables|Default|GetStartCoins))))
      (:NewEnumerator1
        (Variables|Default|SetCurrentAmount _returnvalue))
      (:NewEnumerator2
        (if (!= (Variables|Default|GetStartCoins) (Variables|Default|GetCoins))
          (Variables|Default|SetStartCoins (Variables|Default|GetCoins))
          (Variables|Default|SetStartMeters _returnvalue)
          (Variables|Default|SetCurrentAmount 0)
          (else
            (Variables|Default|SetCurrentAmount (- _returnvalue (Variables|Default|GetStartMeters))))))
      (:NewEnumerator3
        (Variables|Default|SetCurrentAmount (/ (Math|Float|Truncate (Variables|/Game/PixelDrive/Blueprints/CarGamemode.CarGamemode_C|GetSpeed _gamemode)) -2))))))

(fn ConstructionScript)

(fn SavePlayerInfo
  (params (Coins :type Integer) (Highscore :type Integer) (BoughtCars :type Array%20of%20Booleans) (LastCar :type Player%20Car%20Class%20Reference) (Sound :type Float%20%28single-precision%29) (Music :type Float%20%28single-precision%29))
  (bind _returnvalue (SaveGame|CreateSaveGameObject "/Game/PixelDrive/Blueprints/SavePlayer.SavePlayer_C"))
  (bind _output_get (Variables|Default|SetPlayerInfo _returnvalue))
  (Variables|/Game/PixelDrive/Blueprints/SavePlayer.SavePlayer_C|SetCoins _output_get Coins)
  (Variables|/Game/PixelDrive/Blueprints/SavePlayer.SavePlayer_C|SetHighscore _output_get Highscore)
  (Variables|/Game/PixelDrive/Blueprints/SavePlayer.SavePlayer_C|SetBoughtCars _output_get BoughtCars)
  (Variables|/Game/PixelDrive/Blueprints/SavePlayer.SavePlayer_C|SetLastCar _returnvalue LastCar)
  (Variables|/Game/PixelDrive/Blueprints/SavePlayer.SavePlayer_C|SetSVolume _returnvalue Sound)
  (Variables|/Game/PixelDrive/Blueprints/SavePlayer.SavePlayer_C|SetMVolume _returnvalue Music)
  (SaveGame|SaveGametoSlot (Variables|Default|GetPlayerInfo) "PlayerInfo"))

(fn LoadPlayerInfo
  (bind _returnvalue (SaveGame|DoesSaveGameExist "PlayerInfo"))
  (if _returnvalue
    (bind _returnvalue_2 (SaveGame|LoadGamefromSlot "PlayerInfo"))
    (bind _assave_player (Utilities|Casting|CastToSavePlayer _returnvalue_2))
    (bind _output_get (Variables|Default|SetPlayerInfo _assave_player))
    (return (Variables|/Game/PixelDrive/Blueprints/SavePlayer.SavePlayer_C|GetCoins _output_get) (Variables|/Game/PixelDrive/Blueprints/SavePlayer.SavePlayer_C|GetHighscore _output_get) (Variables|/Game/PixelDrive/Blueprints/SavePlayer.SavePlayer_C|GetBoughtCars _output_get) (Variables|/Game/PixelDrive/Blueprints/SavePlayer.SavePlayer_C|GetLastCar _output_get) (Variables|/Game/PixelDrive/Blueprints/SavePlayer.SavePlayer_C|GetSVolume _output_get) (Variables|/Game/PixelDrive/Blueprints/SavePlayer.SavePlayer_C|GetMVolume _output_get))
    (else
      (return 0 0 (Utilities|Array|MakeArray true false false false false) "/Game/PixelDrive/Blueprints/PlayerCar1.PlayerCar1_C" 1.0 1.0))))

(fn Die
  (Game|SetGamePaused true)
  (bind _asgame_hud (Utilities|Casting|CastToGameHud (HUD|GetHUD (Game|GetPlayerController 0))))
  (Variables|/Game/PixelDrive/Blueprints/GameStarted.GameStarted_C|SetPauseMenuVisibility (Variables|/Game/PixelDrive/Blueprints/GameHud.GameHud_C|GetGameStartedWidget _asgame_hud) "Visible")
  (Variables|/Game/PixelDrive/Blueprints/GameStarted.GameStarted_C|SetMenuState (Variables|/Game/PixelDrive/Blueprints/GameHud.GameHud_C|GetGameStartedWidget _asgame_hud) "NewEnumerator1")
  (Widget|SetIsEnabled (Variables|/Game/PixelDrive/Blueprints/GameStarted.GameStarted_C|GetUltraButton (Variables|/Game/PixelDrive/Blueprints/GameHud.GameHud_C|GetGameStartedWidget _asgame_hud)) false)
  (Widget|SetIsEnabled (Variables|/Game/PixelDrive/Blueprints/GameStarted.GameStarted_C|GetLeftButton (Variables|/Game/PixelDrive/Blueprints/GameHud.GameHud_C|GetGameStartedWidget _asgame_hud)) false)
  (Widget|SetIsEnabled (Variables|/Game/PixelDrive/Blueprints/GameStarted.GameStarted_C|GetRightButton (Variables|/Game/PixelDrive/Blueprints/GameHud.GameHud_C|GetGameStartedWidget _asgame_hud)) false)
  (Widget|SetIsEnabled (Variables|/Game/PixelDrive/Blueprints/GameStarted.GameStarted_C|GetPauseButton (Variables|/Game/PixelDrive/Blueprints/GameHud.GameHud_C|GetGameStartedWidget _asgame_hud)) false)
  (Variables|/Game/PixelDrive/Blueprints/GameStarted.GameStarted_C|SetResumeText (Variables|/Game/PixelDrive/Blueprints/GameHud.GameHud_C|GetGameStartedWidget _asgame_hud) "Restart")
  (bind (_coins _highscore _boughtcars _lastcar _sound _music) (CallFunction|LoadPlayerInfo))
  (CallFunction|SavePlayerInfo (Variables|Default|GetCoins) (Variables|Default|GetHighscore) _boughtcars _lastcar _sound _music))