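; PlayerCar3 is a player car variant whose Ultra ability clears traffic and temporarily boosts money earnings.
; The Ultra event marks the quest done, destroys every Car actor, raises the money multiplier, lowers the spawn multiplier and halts car spawning.
; After an UltraDuration delay it re-enables spawning and sets fixed multiplier values, leaving money at double rather than restoring saved values.
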(event EventBeginPlay
  (|CallParentFunction) ; This node is disabled and will not be called.\nDrag off pins to build functionality.
)

(event Collision|EventActorBeginOverlap
  (params (OtherActor :type Actor%20Object%20Reference))
  (|CallParentFunction OtherActor) ; This node is disabled and will not be called.\nDrag off pins to build functionality.
)

(event EventTick
  (params (DeltaSeconds :type Float%20%28single-precision%29))
  (|CallParentFunction DeltaSeconds) ; This node is disabled and will not be called.\nDrag off pins to build functionality.
)

(event EventUltra
  (Variables|Default|SetQuest%20Done true)
  (bind _outactors (Actor|GetAllActorsOfClass "/Game/PixelDrive/Blueprints/Car.Car_C"))
  (for _array_element _outactors
    (Actor|DestroyActor _array_element))
  (Variables|Default|SetMoneyMultiplier 4)
  (Variables|Default|SetSpawnMultiplier 0.1)
  (Variables|Default|SetSpawnCars false)
  (Utilities|FlowControl|Delay (Variables|Default|GetUltraDuration))
  (Variables|Default|SetMoneyMultiplier 2)
  (Variables|Default|SetSpawnMultiplier 1.0)
  (Variables|Default|SetSpawnCars true))

(fn ConstructionScript
  (|CallParentFunction))