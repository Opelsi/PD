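; Game mode for a driving game that tracks car speed, distance travelled and per-biome pacing.
; Tick applies acceleration and a player multiplier to the negative Speed within fixed limits, and accumulates Path.
; ChangeBiom branches on the old biome and speed, cascading to lower tiers from Field through Suburb and Town to City.
; Each tier calls UpdatingBiomeStats, which picks Acceleration and SpawnLength through a NewBiome comparison.
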(event Custom|ChangeBiom
  (bind _speed (Variables|Default|GetSpeed))
  ;[0 1 0.9826] BiomeAccelerationAndCarSpan
  (switch Utilities|FlowControl|Switch|SwitchonBiomes (Variables|Default|GetOldBiome)
    (:NewEnumerator0
      (CallFunction|UpdatingBiomeStats "NewEnumerator0" 2.0 3.2 3.0 3.2 :!label _label))
    (:NewEnumerator1
      (if (<= _speed -2e+02)
        (CallFunction|UpdatingBiomeStats "NewEnumerator0" -1.0 3.2 4.0 3.2 :!label _label_2)
        (else
          (goto _label))))
    (:NewEnumerator2
      (if (<= _speed -2.5e+02)
        (CallFunction|UpdatingBiomeStats "NewEnumerator1" -2.0 3.2 5.0 3.25 :!label _label_3)
        (else
          (goto _label_2))))
    (:NewEnumerator3
      (if (and (<= _speed -3e+02) (>= _speed -6e+02))
        (CallFunction|UpdatingBiomeStats "NewEnumerator2" -4.0 3.2 5.0 3.25)
        (else
          (goto _label_3))))))

(event EventBeginPlay
  ;[0.996 1 0.9301] BeginPlay
  (Variables|Default|SetSpeed -1e+02))

(event EventTick
  (params (DeltaSeconds :type Float%20%28single-precision%29))
  (bind _acceleration (Variables|Default|GetAcceleration))
  (bind _playermultiplier (Variables|Default|GetPlayerMultiplier))
  (bind _returnvalue (* DeltaSeconds _acceleration _playermultiplier))
  ;[1 0 0.8783] Tick:SetUpSpeedAndPath
  (if (and (<= (- (Variables|Default|GetSpeed) _returnvalue) -9e+01) (>= (- (Variables|Default|GetSpeed) _returnvalue) -6e+02))
    (Variables|Default|SetSpeed (- (Variables|Default|GetSpeed) _returnvalue)))
  (Variables|Default|SetPath (+ (Variables|Default|GetPath) (Math|Float|Absolute(Float) (* DeltaSeconds (Variables|Default|GetSpeed) 0.1)) (Math|Float|Absolute(Float) (* _returnvalue DeltaSeconds 0.25)))))

(fn ConstructionScript)

(fn UpdatingBiomeStats
  (params (NewBiome :type Biomes%20Enum :default "NewEnumerator0") (UpperA :type Float%20%28single-precision%29) (UpperS :type Float%20%28single-precision%29) (LowerA :type Float%20%28single-precision%29) (LowerS :type Float%20%28single-precision%29))
  (if (Utilities|Enum|Equal(Enum) (Variables|Default|GetNewBiome) NewBiome)
    (Variables|Default|SetAcceleration UpperA)
    (Variables|Default|SetSpawnLength UpperS)
    (else
      (Variables|Default|SetAcceleration LowerA)
      (Variables|Default|SetSpawnLength LowerS))))