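; Player car Blueprint with an Ultra ability that gives a temporary speed boost.
; Ultra marks the quest done, raises the spawn multiplier and chains two timelines that drive the GameMode's PlayerMultiplier, then resets both multipliers.
; The CrushCol overlap checks the HUD widget's Ulting flag and, while it is set, calls Die on contact with a Car or Obstacle.
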(event OnComponentBeginOverlap(CrushCol)
  (params (OverlappedComponent :type Primitive%20Component%20Object%20Reference) (OtherActor :type Actor%20Object%20Reference) (OtherComp :type Primitive%20Component%20Object%20Reference) (OtherBodyIndex :type Integer) (bFromSweep :type Boolean) (SweepResult :type Hit%20Result%20Structure%20%28by%20ref%29))
  (bind _asgame_hud (Utilities|Casting|CastToGameHud (HUD|GetHUD (Game|GetPlayerController 0))))
  (if (Utilities|IsValid (Variables|/Game/PixelDrive/Blueprints/GameHud.GameHud_C|GetGameStartedWidget _asgame_hud))
    (if (Variables|/Game/PixelDrive/Blueprints/GameStarted.GameStarted_C|GetUlting (Variables|/Game/PixelDrive/Blueprints/GameHud.GameHud_C|GetGameStartedWidget _asgame_hud))
      (Utilities|Casting|CastToCar OtherActor
        (:then
          _)
        (:CastFailed
          (Utilities|Casting|CastToObstacle OtherActor)))
      (CallFunction|Die))))

(event EventBeginPlay
  (|CallParentFunction) ; This node is disabled and will not be called.\nDrag off pins to build functionality.
)

(event Collision|EventActorBeginOverlap
  (params (OtherActor :type Actor%20Object%20Reference))
  (|CallParentFunction OtherActor) ; This node is disabled and will not be called.\nDrag off pins to build functionality.
)

(event EventTick
  (params (DeltaSeconds :type Float%20%28single-precision%29))
  (|CallParentFunction DeltaSeconds) ; This node is disabled and will not be called.\nDrag off pins to build functionality.
)

(event EventUltra
  (bind _gamemode (Variables|Default|GetGameMode))
  (Variables|Default|SetQuest%20Done true)
  (Variables|Default|SetSpawnMultiplier 4.0)
  (bind _acceleration (Timeline|SpeedUp Play)
    (:Update
      (Variables|/Game/PixelDrive/Blueprints/CarGamemode.CarGamemode_C|SetPlayerMultiplier _gamemode _acceleration))
    (:Finished
      (bind _acceleration_2 (Timeline|Timeline_0 Play)
        (:Update
          (Variables|/Game/PixelDrive/Blueprints/CarGamemode.CarGamemode_C|SetPlayerMultiplier _gamemode _acceleration_2))
        (:Finished
          (Variables|/Game/PixelDrive/Blueprints/CarGamemode.CarGamemode_C|SetPlayerMultiplier _gamemode 1.0)
          (Variables|Default|SetSpawnMultiplier 1.0))))))

(fn ConstructionScript
  (|CallParentFunction))